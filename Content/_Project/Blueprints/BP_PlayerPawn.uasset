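; BP_PlayerPawn is a player pawn that acts as a camera rig, with no active gameplay logic in its event graph.
; Its construction script calls ConstructCamera, which rotates the Camera from pitch and rotation variables.
; It then moves the root to an offset point, backed away along the camera's forward vector by a distance.
; An unused asin(1/√3) expression computes the true isometric pitch angle.
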(event EventBeginPlay)

(event Collision|EventActorBeginOverlap
  (params (OtherActor :type Actor%20Object%20Reference)))

(event EventTick
  (params (DeltaSeconds :type Float%20%28single-precision%29)))

(fn ConstructionScript
  (CallFunction|ConstructCamera))

(fn ConstructCamera
  (Transformation|SetRelativeRotation (Variables|Default|GetCamera) (Math|Rotator|MakeRotator 0.0 (* (Variables|CameraSettings|GetcameraPitch) -1.0) (Variables|Default|GetcameraRotation)) false false)
  (Transformation|SetWorldLocation (Variables|Default|GetDefaultSceneRoot) (+ (Variables|CameraSettings|GetcameraOffset) (* (* (Variables|CameraSettings|GetcameraDistance) -1.0) (Math|Vector|GetForwardVector (Variables|Default|GetCamera)))) false false))