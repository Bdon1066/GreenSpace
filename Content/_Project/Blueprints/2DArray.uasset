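; Blueprint 2D array utility that stores a numeric grid in a flat 1D array, using row-major indexing by ArrayWidth.
; ConstructArray zero-fills Width × Height entries, while Get, Set and AddElement read, overwrite or increment single cells.
; AddArray sums another 2D array into this one cell by cell, ignoring its Row and Column inputs and looping rows over the source's width, columns over its height.
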(fn SetElement
  (params (value :type Integer) (row :type Integer) (column :type Integer))
  (Utilities|Array|SetArrayElem (Variables|Default|Get1DArray) (+ column (* row (Variables|Default|GetarrayWidth))) value))

(fn GetElement
  (params (row :type Integer) (column :type Integer))
  (return (Utilities|Array|Get(acopy) (Variables|Default|Get1DArray) (+ column (* row (Variables|Default|GetarrayWidth))))))

(fn ConstructArray
  (for _index (range 0 (- (Variables|Default|GetarrayWidth) 1))
    (for _index_2 (range 0 (- (Variables|Default|GetarrayHeight) 1))
      (Utilities|Array|Add (Variables|Default|Get1DArray) 0))))

(fn AddElement
  (params (value :type Integer) (row :type Integer) (column :type Integer))
  (bind _1darray (Variables|Default|Get1DArray))
  (bind _arraywidth (Variables|Default|GetarrayWidth))
  (bind _returnvalue (* row _arraywidth))
  (bind _returnvalue_2 (+ column _returnvalue))
  (Utilities|Array|SetArrayElem _1darray _returnvalue_2 (+ (Utilities|Array|Get(acopy) _1darray _returnvalue_2) value)))

(fn AddArray
  (params (row :type Integer) (column :type Integer) (array :type 2D%20Array%20Object%20Reference))
  (for _index (range 0 (- (Variables|2DArray_C|GetarrayWidth array) 1))
    (for _index_2 (range 0 (- (Variables|2DArray_C|GetarrayHeight array) 1))
      (bind _value (CallFunction|GetElement array _index _index_2))
      (CallFunction|AddElement _value _index _index_2))))