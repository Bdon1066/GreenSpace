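; Player controller that handles mouse selection of grid cells, with a debug check for placement next to the clicked cell.
; On begin play it shows the cursor and adds the player input mapping context.
; Each click traces under the cursor to a BP_Grid, caches that grid on first hit, and selects and returns the hit component's cell index.
; The grid's neighbour lookup then decides whether placement to the right is printed as possible.
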(event Input|EnhancedActionEvents|EnhancedInputActionIA_Click
  (params (ActionValue :type Boolean) (ElapsedSeconds :type Float%20%28double-precision%29) (TriggeredSeconds :type Float%20%28double-precision%29) (InputAction :type Input%20Action%20Object%20Reference :default "/Game/_Project/Input/IA_Click.IA_Click"))
  (:Started
    (bind _index (CallFunction|GetGridCellUnderCursor))
    (bind _isvalid (Default|GetNeighbouringCell (Variables|Default|GetGrid) _index "NewEnumerator3"))
    (if _isvalid
      (Development|PrintString "Can place to RIGHT of this cell")
      (else
        (Development|PrintString "CANNOT place to RIGHT of this cell")))))

(event EventBeginPlay
  (Variables|Default|SetbShowMouseCursor true)
  (Input|AddMappingContext (PlayerController|LocalPlayerSubsystems|GetEnhancedInputLocalPlayerSubsystem) "/Game/_Project/Input/IMC_Player.IMC_Player" 0 "(bIgnoreAllPressedKeysUntilRelease=True,bForceImmediately=False,bNotifyUserSettings=False)"))

(event EventTick
  (params (DeltaSeconds :type Float%20%28single-precision%29)))

(fn ConstructionScript)

(fn GetGridCellUnderCursor
  (bind _array (Utilities|Array|MakeArray "ObjectTypeQuery1" "ObjectTypeQuery2"))
  (bind _hitresult (Class|PlayerController|GetHitResultUnderCursorforObjects _array true))
  (bind (_bblockinghit _binitialoverlap _time _distance _location _impactpoint _normal _impactnormal _physmat _hitactor _hitcomponent) (Collision|BreakHitResult _hitresult))
  (bind _asbp_grid (Utilities|Casting|CastToBP_Grid _hitactor))
  (Utilities|IsValid (Variables|Default|GetGrid)
    (:Is%20Valid
      _)
    (:Is%20Not%20Valid
      (bind _output_get (Variables|Default|SetGrid _asbp_grid))))
  (Default|SelectCell (Variables|Default|GetGrid) (Default|GetIndexfromCell _output_get _hitcomponent))
  (return (Default|GetIndexfromCell _output_get _hitcomponent)))