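; Grid actor that builds a field of static mesh cells and can stamp predefined block shapes onto it.
; The construction script spawns the cells, a 2DArray math grid (rebuilt on every cell iteration) and rectangular and L shape templates.
; PlaceShape adds a template into the grid, then UpdateGrid paints occupied cells red; nothing live calls it.
; Neighbour lookups use index offsets and modulo edge checks based only on Rows.
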(event EventBeginPlay)

(fn ConstructionScript
  (CallFunction|CreateGrid)
  (CallFunction|CreateShapes))

(fn CreateGrid
  (for _index (range 0 (- (Variables|Default|Getrows) 1))
    (for _index_2 (range 0 (- (Variables|Default|Getcolumns) 1))
      (bind _returnvalue (AddComponent|AddStaticMeshComponent false (Math|Transform|MakeTransform (Math|Vector|MakeVector (* _index_2 (Variables|Default|GetcellSize)) (* _index (Variables|Default|GetcellSize)) 0.0) "0, 0, 0" (Variables|Default|GetcellCubeScale))))
      (Utilities|Array|Add (Variables|Default|Getcells) _returnvalue)
      ;[1 1 1] math array for grid
      (bind _returnvalue_2 (Game|ConstructObjectfromClass "/Game/_Project/Blueprints/2DArray.2DArray_C" 0 (Variables|Default|Getrows) (Variables|Default|Getcolumns)))
      (bind _output_get (Variables|Default|SetGrid _returnvalue_2))
      (Default|ConstructArray _output_get))))

(fn GetNeighbouringCell
  (params (cellIndex :type Integer) (direction :type E_Direction%20Enum :default "NewEnumerator0"))
  (bind _output_get (LocalVariables|SetcurrentCell cellIndex))
  (switch Utilities|FlowControl|Switch|SwitchonE_Direction direction
    (:NewEnumerator0
      ;[1 1 1] n -1 (Left)
      (LocalVariables|SetneighbouringCell (+ _output_get -1))
      (Utilities|Is(currentCell)/RowsNOTMod0?))
    (:NewEnumerator1
      ;[1 1 1] n + 1 (Right)
      (LocalVariables|SetneighbouringCell (+ _output_get 1))
      (Utilities|Is(currentCell+1)/RowsNOTMod0?))
    (:NewEnumerator2
      ;[1 1 1] n + r (Top)
      (LocalVariables|SetneighbouringCell (+ _output_get (Variables|Default|Getrows)))
      (Utilities|IsCurrentCellNOT<Rows?))
    (:NewEnumerator3
      ;[1 1 1] n - r (Bottom)
      (LocalVariables|SetneighbouringCell (+ _output_get (* -1 (Variables|Default|Getrows))))
      (Utilities|IsCurrentCellNOT>=RowsX(rows-1)?)))
  (return (LocalVariables|GetneighbouringCell) (LocalVariables|Getvalid)))

(fn GetIndexfromCell
  (params (Cell :type Primitive%20Component%20Object%20Reference))
  (return (Utilities|Array|FindItem (Variables|Default|Getcells) Cell)))

(fn SelectCell
  (params (index :type Integer))
  (Rendering|Material|SetMaterial (Utilities|Array|Get(acopy) (Variables|Default|Getcells) index) 0 "/Game/_Project/Materials/M_Red.M_Red")
  (Utilities|Array|Add (Variables|Default|GetselectedCells) index))

(fn GetNeighbouringCells
  (params (index :type Integer) (neighbouringCells :type Array%20of%20E_Direction%20Enums :default "NewEnumerator0"))
  (bind _array_element (Utilities|Array|ForEachLoopwithBreak neighbouringCells :!label _label)
    (:LoopBody
      (bind _isvalid (CallFunction|GetNeighbouringCell index _array_element))
      (if (not _isvalid)
        (goto _label Break)))))

(fn CreateShapes
  ;[1 1 1] 1x2
  (bind _returnvalue (Game|ConstructObjectfromClass "/Game/_Project/Blueprints/2DArray.2DArray_C" (Utilities|Array|MakeArray 1 1) 2 1))
  (Default|ConstructArray _returnvalue)
  (Utilities|Array|Add (Variables|Default|GetShapes) _returnvalue)
  ;[1 1 1] 1x3
  (bind _returnvalue_2 (Game|ConstructObjectfromClass "/Game/_Project/Blueprints/2DArray.2DArray_C" (Utilities|Array|MakeArray 1 1 1) 1 3))
  (Default|ConstructArray _returnvalue_2)
  (Utilities|Array|Add (Variables|Default|GetShapes) _returnvalue_2)
  ;[1 1 1] 1x4
  (bind _returnvalue_3 (Game|ConstructObjectfromClass "/Game/_Project/Blueprints/2DArray.2DArray_C" (Utilities|Array|MakeArray 1 1 1 1) 1 4))
  (Default|ConstructArray _returnvalue_3)
  (Utilities|Array|Add (Variables|Default|GetShapes) _returnvalue_3)
  ;[1 1 1] 2x2
  (bind _returnvalue_4 (Game|ConstructObjectfromClass "/Game/_Project/Blueprints/2DArray.2DArray_C" (Utilities|Array|MakeArray 1 1 1 1) 2 2))
  (Default|ConstructArray _returnvalue_4)
  (Utilities|Array|Add (Variables|Default|GetShapes) _returnvalue_4)
  ;[1 1 1] 2x3
  (bind _returnvalue_5 (Game|ConstructObjectfromClass "/Game/_Project/Blueprints/2DArray.2DArray_C" (Utilities|Array|MakeArray 1 1 1 1 1 1) 2 3))
  (Default|ConstructArray _returnvalue_5)
  (Utilities|Array|Add (Variables|Default|GetShapes) _returnvalue_5)
  ;[1 1 1] 2x4
  (bind _returnvalue_6 (Game|ConstructObjectfromClass "/Game/_Project/Blueprints/2DArray.2DArray_C" (Utilities|Array|MakeArray 1 1 1 1 1 1 1 1) 2 4))
  (Default|ConstructArray _returnvalue_6)
  (Utilities|Array|Add (Variables|Default|GetShapes) _returnvalue_6)
  ;[1 1 1] 3x3
  (bind _returnvalue_7 (Game|ConstructObjectfromClass "/Game/_Project/Blueprints/2DArray.2DArray_C" (Utilities|Array|MakeArray 1 1 1 1 1 1 1 1 1) 3 3))
  (Default|ConstructArray _returnvalue_7)
  (Utilities|Array|Add (Variables|Default|GetShapes) _returnvalue_7)
  ;[1 1 1] L Shape
  (bind _returnvalue_8 (Game|ConstructObjectfromClass "/Game/_Project/Blueprints/2DArray.2DArray_C" (Utilities|Array|MakeArray 1 1 1 0 0 1) 3 2))
  (Default|ConstructArray _returnvalue_8)
  (Utilities|Array|Add (Variables|Default|GetShapes) _returnvalue_8))

(fn GetShape
  (params (enum :type E_Shapes%20Enum :default "NewEnumerator6"))
  (return (Utilities|Array|Get(acopy) (Variables|Default|GetShapes) (Math|Conversions|ToInteger(Byte) enum))))

(fn UpdateGrid
  (for (_array_element _array_index) (Variables|/Game/_Project/Blueprints/2DArray.2DArray_C|Get1DArray (Variables|Default|GetGrid))
    (if (>= _array_element 1)
      (CallFunction|SelectCell _array_index))))

(fn PlaceShape
  (params (enum :type E_Shapes%20Enum :default "NewEnumerator6") (index :type Integer))
  (bind _grid (Variables|Default|GetGrid))
  (bind _shape (CallFunction|GetShape enum))
  (bind (_x _y) (Default|Get2DIndices _grid index))
  (Default|AddArray _grid _x _y _shape)
  (CallFunction|UpdateGrid))